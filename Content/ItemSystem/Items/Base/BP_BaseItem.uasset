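; BP_BaseItem is a base item Blueprint with equip, unequip and use events.
; Each event prints the action with the item's DisplayName.
; Use also restarts SpinTimeline, whose Rotation track drives both roll and yaw of the static mesh's relative rotation.
; BeginPlay, overlap, Tick and the construction script hold no logic.
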(event EventBeginPlay)

(event Collision|EventActorBeginOverlap
  (params (OtherActor :type Actor%20Object%20Reference)))

(event EventTick
  (params (DeltaSeconds :type Float%20%28single-precision%29)))

(event EventOnUnequip
  (Development|PrintString (Utilities|String|Append "Unequipped: " (Utilities|String|ToString(Text) (Variables|Default|GetDisplayName)))))

(event EventOnEquip
  (Development|PrintString (Utilities|String|Append "Equipped: " (Utilities|String|ToString(Text) (Variables|Default|GetDisplayName)))))

(event EventOnUse
  (Development|PrintString (Utilities|String|Append "Used: " (Utilities|String|ToString(Text) (Variables|Default|GetDisplayName))))
  (bind _rotation (Timeline|SpinTimeline PlayFromStart)
    (:Update
      (Transformation|SetRelativeRotation (Variables|Default|GetStaticMesh) (Math|Rotator|MakeRotator _rotation 0.0 _rotation) false false))))

(fn ConstructionScript)